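; EscaCube is a Blueprint that shuttles a cube back and forth along a spline path.
; Each Tick advances or retreats a stored distance at constant, frame-rate-independent speed and places the Cube at that point on LescaSpline in local space, without sweeping.
; The Reverse flag flips at each end of the spline; despite its name, the cube moves toward the last point while it is true.
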(event `self.ReceiveTick`
  (params (DeltaSeconds :type "Float (single-precision)"))
  (bind _returnvalue (* 500 DeltaSeconds))
  (bind _l_escaspline (`self.L'escaSpline`))
  (bind _cube (`self.Cube`))
  (if (`self.Reverse`)
    (bind _output_get (set `self.Distance` (+ _returnvalue (`self.Distance`))))
    (`SceneComponent.K2_SetRelativeLocation` _cube (`SplineComponent.GetLocationAtDistanceAlongSpline` _l_escaspline _output_get "Local") false false)
    (if (>= _output_get (`SplineComponent.GetDistanceAlongSplineAtSplinePoint` _l_escaspline (- (`SplineComponent.GetNumberOfSplinePoints` _l_escaspline) 1)))
      (set `self.Reverse` false))
    (else
      (bind _output_get_2 (set `self.Distance` (- (`self.Distance`) _returnvalue)))
      (`SceneComponent.K2_SetRelativeLocation` _cube (`SplineComponent.GetLocationAtDistanceAlongSpline` _l_escaspline _output_get_2 "Local") false false)
      (if (<= _output_get_2 0.0)
        (set `self.Reverse` true)))))

(fn `UserConstructionScript`)